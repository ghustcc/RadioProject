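; BP_Radio is an interactive radio actor that toggles on and off and tunes through a clamped FM frequency range.
; It starts off, and each toggle plays an on or off montage and shows or hides the FM and station texts.
; While on, tuning input steps the frequency, updates a child TextRenderActor, rotates the dial and clicks whenever the value changes.
; The music play and stop functions are empty stubs.
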(event `self.ReceiveBeginPlay`
  (`self.TurnRadioOff`))

(event `self.ReceiveTick`
  (params (DeltaSeconds :type "Float (single-precision)")))

(event `TurnRadioOn`
  (`|PlayMontage` (`self.Radio`) "/Game/Art/Animations/AM_RadioOn.AM_RadioOn"
    (:`then`
      (`SceneComponent.SetVisibility` (`self.FMText`) true false)
      (`SceneComponent.SetVisibility` (`self.RadioStationText`) true false)
      (`self.ChangeRadioStationText` (`self.CurrentRadioStation`))
      (set `self.RadioIsOn` true))))

(event `TurnRadioOff`
  (`|PlayMontage` (`self.Radio`) "/Game/Art/Animations/AM_RadioOff.AM_RadioOff"
    (:`then`
      (`SceneComponent.SetVisibility` (`self.FMText`) false false)
      (`SceneComponent.SetVisibility` (`self.RadioStationText`) false false)
      (set `self.RadioIsOn` false))))

(event `ToggleRadioOnOff`
  (if (`self.RadioIsOn`)
    (`self.TurnRadioOff`)
    (else
      (`self.TurnRadioOn`))))

(event `ChangeRadioStation`
  (params (`Input Value` :type "Float (double-precision)"))
  (if (`self.RadioIsOn`)
    (bind _output_get (set `self.CurrentRadioStation` (`KismetMathLibrary.FClamp` (+ (`self.CurrentRadioStation`) (* 0.5 `Input Value`)) 101.5 109.5)))
    (if (!= _output_get (`self.LastRadioStation`))
      (set `self.LastRadioStation` (`self.CurrentRadioStation`))
      (`self.ChangeRadioStationText` (`self.CurrentRadioStation`))
      (`SceneComponent.K2_AddRelativeRotation` (`self.Radio Station Spin`) (`KismetMathLibrary.MakeRotator` 0.0 (* -2.0 `Input Value`)) false false)
      (`GameplayStatics.PlaySound2D` "/Engine/VREditor/Sounds/UI/Click_on_Button.Click_on_Button" 1.0 1.0 0.0 null null))))

(fn `ChangeRadioStationText`
  (params (Station :type "Float (double-precision)"))
  (bind _astext_render_actor (cast `TextRenderActor` (`ChildActorComponent.ChildActor` (`self.RadioStationText`))))
  (`TextRenderComponent.K2_SetText` (`TextRenderActor.TextRender` _astext_render_actor) (`|FormatText` (`KismetTextLibrary.Conv_DoubleToText` Station "HalfToEven" false true 1 324 1))))

(fn `PlayMusicRadio`)

(fn `StopMusicRadio`)

(fn `UserConstructionScript`)