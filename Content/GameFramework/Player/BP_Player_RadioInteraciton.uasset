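; Player pawn for looking at and interacting with a radio, with mouse-look style camera control and FOV zoom.
; BeginPlay adds the radio Enhanced Input mapping context, whose actions drive controller yaw/pitch and clamped camera zoom.
; Every tick, a short debug-drawn line trace from the camera stores the hit actor as HitRadio and prints the component name.
; Interaction input only prints its value, station change is an empty stub, and ExecuteZoomPayer is never called.
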(event `self.ReceiveBeginPlay`
  (`EnhancedInputSubsystemInterface.AddMappingContext` (pcsubsystem `EnhancedInputLocalPlayerSubsystem` (`GameplayStatics.GetPlayerController` 0)) "/Game/Input/IMC_RadioInteration.IMC_RadioInteration" 0 (struct)))

(event `self.ReceiveTick`
  (params (DeltaSeconds :type "Float (single-precision)"))
  (`self.ExecuteLineTracing`))

(event `EnhancedInput|/Game/Input/IA_RadioInteraction`
  (params (ActionValue :type Boolean) (ElapsedSeconds :type "Float (double-precision)") (TriggeredSeconds :type "Float (double-precision)") (InputAction :type "InputAction Object Reference" :default "/Game/Input/IA_RadioInteraction.IA_RadioInteraction"))
  (:`Triggered`
    (`KismetSystemLibrary.PrintString` (`KismetStringLibrary.Conv_BoolToString` ActionValue))))

(event `EnhancedInput|/Game/Input/IA_ChangeRadioStation`
  (params (ActionValue :type "Float (double-precision)") (ElapsedSeconds :type "Float (double-precision)") (TriggeredSeconds :type "Float (double-precision)") (InputAction :type "InputAction Object Reference" :default "/Game/Input/IA_ChangeRadioStation.IA_ChangeRadioStation")))

(event `EnhancedInput|/Game/Input/IA_CameraMoviment`
  (params (ActionValue :type "Vector2D Structure") (ElapsedSeconds :type "Float (double-precision)") (TriggeredSeconds :type "Float (double-precision)") (InputAction :type "InputAction Object Reference" :default "/Game/Input/IA_CameraMoviment.IA_CameraMoviment"))
  (:`Triggered`
    (`self.AddControllerYawInput` ActionValue_X)
    (`self.AddControllerPitchInput` (* ActionValue_Y -1.0))))

(event `EnhancedInput|/Game/Input/IA_PlayerZoom`
  (params (ActionValue :type "Float (double-precision)") (ElapsedSeconds :type "Float (double-precision)") (TriggeredSeconds :type "Float (double-precision)") (InputAction :type "InputAction Object Reference" :default "/Game/Input/IA_PlayerZoom.IA_PlayerZoom"))
  (:`Triggered`
    (bind _output_get (set `self.ZoomAmount` ActionValue))
    (`CameraComponent.SetFieldOfView` (`self.Camera`) (`KismetMathLibrary.FClamp` (- (`CameraComponent.FieldOfView` (`self.Camera`)) (* _output_get (`self.SpeedZoom`))) 30.0 90.0))))

(fn `ExecuteLineTracing`
  (bind _camera (`self.Camera`))
  (bind _returnvalue (`SceneComponent.K2_GetComponentLocation` _camera))
  (bind (_outhit _returnvalue_2) (`KismetSystemLibrary.LineTraceSingle` :`Start` _returnvalue :`End` (+ _returnvalue (* (`SceneComponent.GetForwardVector` _camera) 200.0)) :`TraceChannel` "TraceTypeQuery1" :`DrawDebugType` "ForOneFrame"))
  (if _returnvalue_2
    (set `self.HitRadio` (`.HitActor` (`GameplayStatics.BreakHitResult` _outhit)))
    (`KismetSystemLibrary.PrintString` (`KismetSystemLibrary.GetDisplayName` (`.HitComponent` (`GameplayStatics.BreakHitResult` _outhit))))))

(fn `ExecuteZoomPayer`
  (bind _output_get (set `self.ZoomAmount` 0.0))
  (`CameraComponent.SetFieldOfView` (`self.Camera`) (`KismetMathLibrary.FClamp` (- (`CameraComponent.FieldOfView` (`self.Camera`)) (* _output_get 5.0)) 300.0 90.0)))

(fn `UserConstructionScript`)